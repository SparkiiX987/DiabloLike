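; Dungeon game mode that tracks living enemies and moves the game to a win level once all are dead.
; On BeginPlay it starts the dungeon, gathers every C_BaseEnemy actor into a list and caches the player character.
; Each OnEnemyDeath call removes that enemy, then either opens the win level or sends the remaining count to the player for display.
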(event Custom|OnEnemyDeath
  (params (Item :type C%20Base%20Enemy%20Object%20Reference%20%28by%20ref%29))
  (bind _enemies (Variables|Default|GetEnemies))
  (bind _returnvalue (Utilities|Array|Length _enemies))
  (Utilities|Array|RemoveItem _enemies Item)
  (if (== _returnvalue 0)
    (Game|OpenLevel(byObjectReference) "/Game/Levels/WinLevel.WinLevel")
    (else
      (Default|UpdateEnemiesCount (Variables|Default|GetPlayer) (Utilities|Text|ToText(Integer) _returnvalue)))))

(event EventBeginPlay
  (Class|DungeonGamemode|StartDungeon)
  (bind _outactors (Actor|GetAllActorsOfClass "/Game/Characters/Enemies/BaseEnemy/C_BaseEnemy.C_BaseEnemy_C"))
  (Variables|Default|SetEnemies _outactors)
  (bind _asc_player (Utilities|Casting|CastToC_Player (Game|GetPlayerCharacter 0)))
  (Variables|Default|SetPlayer _asc_player)
  (Default|UpdateEnemiesCount (Variables|Default|GetPlayer) (Utilities|Text|ToText(Integer) (Utilities|Array|Length (Variables|Default|GetEnemies)))))

(fn ConstructionScript)